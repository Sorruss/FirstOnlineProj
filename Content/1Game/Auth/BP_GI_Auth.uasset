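; Game instance Blueprint that handles PlayFab account sign-up, email login and password recovery.
; On init it sets the PlayFab title and, if a save slot exists, skips straight to the post-login level; otherwise it creates an auth save object, which is never written here.
; Successful registration or login opens that level with game-only input, while recovery success just prints a message.
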(event Custom|ForgotPassword
  (params (Email :type String))
  ;[0.15 0.15 0.15 0.5] Forgot Password Logic
  (|SendAccountRecoveryEmail (Utilities|Struct|MakeAdminSendAccountRecoveryEmailRequest 0 Email) (delegate Custom|OnForgotPasswordSuccess) (EventDispatchers|CreateEvent :!event Custom|OnFail)))

(event Custom|SignUp
  (params (Username :type String) (Email :type String) (Password :type String))
  ;[0.15 0.15 0.15 0.5] Registration Logic
  (|RegisterPlayFabUser (Utilities|Struct|MakeClientRegisterPlayFabUserRequest 0 Username Email "" 0 Password "" false Username) (EventDispatchers|CreateEvent :!event Custom|OnRegisterSuccess) (EventDispatchers|CreateEvent :!event Custom|OnFail)))

(event Custom|LogIn
  (params (Email :type String) (Password :type String))
  ;[0.15 0.15 0.15 0.5] Login Logic
  (|LoginwithEmailAddress (Utilities|Struct|MakeClientLoginWithEmailAddressRequest 0 Email 0 Password) (EventDispatchers|CreateEvent :!event Custom|OnLoginSuccess) (EventDispatchers|CreateEvent :!event Custom|OnFail)))

(event Custom|OnFail
  (params (error :type Play%20Fab%20Error%20Structure) (customData :type Object%20Object%20Reference))
  ;[0.15 0.15 0.15 0.5] Helpers
  (Development|PrintString (Utilities|String|Append (.errorname error) ": " (.errormessage error) "(" (.errordetails error) ")") true true "(R=0.000000,G=0.660000,B=1.000000,A=1.000000)" 3e+01))

(event Custom|OnRegisterSuccess
  (params (result :type Client%20Register%20Play%20Fab%20User%20Result%20Structure) (customData :type Object%20Object%20Reference))
  ;[0.15 0.15 0.15 0.5] Helpers
  (CallFunction|OnSuccess))

(event Custom|OnLoginSuccess
  (params (result :type Client%20Login%20Result%20Structure) (customData :type Object%20Object%20Reference))
  ;[0.15 0.15 0.15 0.5] Helpers
  (CallFunction|OnSuccess))

(event Custom|OnForgotPasswordSuccess
  (params (result :type Admin%20Send%20Account%20Recovery%20Email%20Result%20Structure) (customData :type Object%20Object%20Reference))
  ;[0.15 0.15 0.15 0.5] Forgot Password Logic
  (Development|PrintString "Email was send." true true "(R=0.000000,G=0.660000,B=1.000000,A=1.000000)" 1e+01))

(event EventInit
  (Class|PlayFabUtilities|SetPlayFabSettings (Variables|Default|GetGame%20Title%20Id))
  (bind _returnvalue (SaveGame|DoesSaveGameExist (Variables|Default|GetGameSaveSlotName)))
  (if _returnvalue
    (CallFunction|OnSuccess)
    (else
      (bind _returnvalue_2 (SaveGame|CreateSaveGameObject "/Game/1Game/Auth/BP_SG_UserAuthData.BP_SG_UserAuthData_C"))
      (Variables|Default|SetNewSGO _returnvalue_2))))

(fn OnSuccess
  (Game|OpenLevel(byObjectReference) (Variables|Default|GetLevelAfterLoginSuccess))
  (Input|SetInputModeGameOnly (Game|GetPlayerController 0) false))