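; SaveGame object that stores user auth data (username, PlayFab ID, last login time) and decides whether a login is recent enough for auto-login.
; AssignData replaces the record and UpdateData refreshes only the login time, each saving itself to the "UAD" slot.
; CheckIfLoginRecently parses the day from the timestamp string and compares its difference from today against AutoLoginWindowDays, ignoring month and year.
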(fn AssignData
  (params (Data :type S%20User%20Auth%20Data%20Structure))
  (Variables|Default|SetUserData Data)
  (SaveGame|SaveGametoSlot self "UAD"))

(fn CheckifLoginRecently
  (return (< (* (- (Math|Conversions|ToInteger(Byte) (.RightS (Utilities|String|Split (.RightS (Utilities|String|Split (.LeftS (Utilities|String|Split (Utilities|Struct|BreakS_UserAuthData (Variables|Default|GetUserData)) "T")) "-")) "-"))) (Class|KismetMathLibrary|GetDay (Math|DateTime|Now))) -1) (Variables|Default|GetAutoLoginWindowDays))))

(fn UpdateData
  (params (User%20Data%20Last%20Login%20Time :type String))
  (Variables|Default|SetUserData (Utilities|Struct|MakeS_UserAuthData (.username (Variables|Default|GetUserData)) (.playfabid (Variables|Default|GetUserData)) User%20Data%20Last%20Login%20Time))
  (SaveGame|SaveGametoSlot self "UAD"))