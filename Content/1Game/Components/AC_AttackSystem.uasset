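; Melee attack component for BP_YukoPawn that handles weapon equipping, attacks and hit detection.
; Montage notifies move the weapon between hand and spine sockets and release the attack lock; attacking while unarmed equips first.
; Attack montages are indexed by a combo count that resets after a retriggerable delay.
; A looping timer line-traces socket paths plus cross-socket diagonals, damaging each actor once per swing with a computed hit direction.
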(event Custom|WeaponTracing
  (bind _weaponsocketlastlocation (Variables|Tracing|GetWeaponSocketLastLocation))
  (bind _character (Variables|Default|GetCharacter))
  (bind _weaponsocketlastlastlocation (Variables|Tracing|GetWeaponSocketLastLastLocation))
  (bind _array (Utilities|Array|MakeArray _character))
  ;[0.15 0.15 0.15 0.5] Socket Sword Tracing + Calculating Hit Direction
  (bind _keys (Utilities|Map|Keys _weaponsocketlastlocation))
  (for (_array_element _array_index) _keys
    (Variables|Tracing|SetIsThisFirstSocket? (== 0 _array_index))
    (bind (_outhits _returnvalue) (Collision|MultiLineTraceByChannel (.Value (Utilities|Map|Find _weaponsocketlastlocation _array_element)) (Transformation|GetSocketLocation (Variables|/Game/1Game/Weapons/BP_Base_SWeapon.BP_Base_SWeapon_C|GetWeapon (Variables|Default|GetWeaponActor)) _array_element) "TraceTypeQuery3" false _array (Variables|Tracing|GetDrawDebugTraces?)))
    (Variables|Tracing|SetHittedActorsFirstTrace _outhits)
    (if (Variables|Tracing|GetIsThisFirstSocket?)
      _
      (else
        (bind _keys_2 (Utilities|Map|Keys _weaponsocketlastlastlocation))
        (bind (_outhits_2 _returnvalue_2) (Collision|MultiLineTraceByChannel (.Value (Utilities|Map|Find _weaponsocketlastlastlocation (Utilities|Array|Get(acopy) _keys_2 (- _array_index 1)))) (.Value (Utilities|Map|Find _weaponsocketlastlocation _array_element)) "TraceTypeQuery3" false _array (Variables|Tracing|GetDrawDebugTraces?)))
        (Variables|Tracing|SetHittedActorsSecondTrace _outhits_2)
        (Utilities|Map|Add (Variables|Tracing|GetWeaponSocketLastLastLocation) (Utilities|Array|Get(acopy) _keys_2 (- _array_index 1)) (.Value (Utilities|Map|Find (Variables|Tracing|GetWeaponSocketLastLocation) (Utilities|Array|Get(acopy) _keys_2 (- _array_index 1)))))))
    (Utilities|Map|Add (Variables|Tracing|GetWeaponSocketLastLocation) _array_element (Transformation|GetSocketLocation (Variables|/Game/1Game/Weapons/BP_Base_SWeapon.BP_Base_SWeapon_C|GetWeapon (Variables|Default|GetWeaponActor)) _array_element))
    (if (or _returnvalue _returnvalue_2)
      (Utilities|Array|AppendArray (Variables|Tracing|GetHittedActorsFirstTrace) (Variables|Tracing|GetHittedActorsSecondTrace))
      (for _array_element_2 (Variables|Tracing|GetHittedActorsFirstTrace)
        (if (not (Utilities|Array|ContainsItem (Variables|Tracing|GetAlreadyHittedActors) (.HitActor (Collision|BreakHitResult _array_element_2))))
          (Utilities|Array|Add (Variables|Tracing|GetAlreadyHittedActors) (.HitActor (Collision|BreakHitResult _array_element_2)))
          (Class|BPIDamageSystem|TakeDamage(Message) (.HitActor (Collision|BreakHitResult _array_element_2)) (Utilities|Struct|MakeS_DamageInfo (Variables|Default|GetCharacter) (Variables|/Game/1Game/Weapons/BP_Base_SWeapon.BP_Base_SWeapon_C|GetDamage (Variables|Default|GetWeaponActor)) true true true false (CallFunction|GetDirectionOfAnotherActor (.HitActor (Collision|BreakHitResult _array_element_2)) (Variables|Default|GetCharacter)))))))))

(event Custom|EquipWeapon
  (bind _character (Variables|Default|GetCharacter))
  ;[0.15 0.15 0.15 0.5] Equip and Dequip Weapon Logic
  (if (not (Variables|States|GetIsWeaponEquipped?))
    (bind _notifyname (Animation|Montage|PlayMontage (Variables|/Script/Engine.Character|GetMesh (Variables|Default|GetCharacter)) "/Game/YukoProject/Character/Animations/Combat/Equip_Montage.Equip_Montage")
      (:OnNotifyBegin
        (switch name _notifyname
          (:Equipped
            (Transformation|AttachComponentToComponent (Variables|/Game/YukoProject/Character/Blueprints/BP_YukoPawn.BP_YukoPawn_C|GetActiveWeaponActor _character) (Variables|/Game/YukoProject/Character/Blueprints/BP_YukoPawn.BP_YukoPawn_C|Gethandsocket_scene _character) "None" "SnapToTarget" "SnapToTarget" "SnapToTarget" true)
            (CallFunction|AfterEquip)))))))

(event Custom|DequipWeapon
  (bind _character (Variables|Default|GetCharacter))
  ;[0.15 0.15 0.15 0.5] Equip and Dequip Weapon Logic
  (if (and (Variables|States|GetIsWeaponEquipped?) (not (Variables|States|GetDequipAlreadyStarted?)))
    (bind _notifyname (Animation|Montage|PlayMontage (Variables|/Script/Engine.Character|GetMesh (Variables|Default|GetCharacter)) "/Game/YukoProject/Character/Animations/Combat/Unequip_Montage.Unequip_Montage")
      (:then
        (Variables|States|SetDequipAlreadyStarted? true))
      (:OnNotifyBegin
        (switch name _notifyname
          (:Unequipped
            (Transformation|AttachComponentToComponent (Variables|/Game/YukoProject/Character/Blueprints/BP_YukoPawn.BP_YukoPawn_C|GetActiveWeaponActor _character) (Variables|/Game/YukoProject/Character/Blueprints/BP_YukoPawn.BP_YukoPawn_C|Getspinesocket_scene _character) "None" "SnapToTarget" "SnapToTarget" "SnapToTarget" true)
            (CallFunction|AfterDequip)))))))

(event Custom|MontageWithTrace
  (bind _character (Variables|Default|GetCharacter))
  ;[0.15 0.15 0.15 0.5] Attack Montage Player
  (if (not (Variables|States|GetAttackAlreadyStarted?))
    (Default|CallPlayerAttack)
    (bind _notifyname (Animation|Montage|PlayMontage (Variables|/Script/Engine.Character|GetMesh (Variables|Default|GetCharacter)) (Utilities|Array|Get(acopy) (Variables|/Game/1Game/Weapons/BP_Base_SWeapon.BP_Base_SWeapon_C|GetAttackMontages (Variables|Default|GetWeaponActor)) (Variables|Default|GetComboCount)))
      (:then
        (Default|SetAnimationLock _character true)
        (Variables|States|SetAttackAlreadyStarted? true))
      (:OnInterrupted
        (Default|SetAnimationLock _character false :!label _label)
        (Variables|States|SetAttackAlreadyStarted? false))
      (:OnNotifyBegin
        (switch name _notifyname
          (:AnimationLockOff
            (goto _label)))))))

(event Custom|WeaponTraceStart
  ;[0.15 0.15 0.15 0.5] Socket Sword Tracing + Calculating Hit Direction
  (CallFunction|UpdateWeaponSockets)
  (bind _returnvalue (Utilities|Time|SetTimerbyEvent (delegate Custom|WeaponTracing) (Variables|Tracing|GetTracingEveryNTime) true)))

(event Custom|WeaponTraceEnd
  ;[0.15 0.15 0.15 0.5] Socket Sword Tracing + Calculating Hit Direction
  (if (Utilities|Time|IsValidTimerHandle (stale Custom|WeaponTraceStart _returnvalue))
    (Utilities|Time|ClearandInvalidateTimerbyHandle (stale Custom|WeaponTraceStart _returnvalue))
    (Utilities|Array|Clear (Variables|Tracing|GetAlreadyHittedActors))))

(event Custom|Attack
  (if (Variables|States|GetIsWeaponEquipped?)
    (CallFunction|MontagewithTrace)
    (Utilities|FlowControl|RetriggerableDelay (Variables|Default|GetComboWindow))
    (Variables|Default|SetComboCount 0)
    (else
      (CallFunction|EquipWeapon))))

(event EventBeginPlay
  (bind _asbp_yuko_pawn (Utilities|Casting|CastToBP_YukoPawn (Components|GetOwner)))
  (bind _output_get (Variables|Default|SetCharacter _asbp_yuko_pawn))
  (Utilities|FlowControl|DelayUntilNextTick)
  (Variables|Default|SetWeaponActor (Variables|/Game/YukoProject/Character/Blueprints/BP_YukoPawn.BP_YukoPawn_C|GetActiveWeaponActor _output_get)))

(fn UpdateWeaponSockets
  (bind _weaponactor (Variables|Default|GetWeaponActor))
  (for _array_element (Variables|/Game/1Game/Weapons/BP_Base_SWeapon.BP_Base_SWeapon_C|GetSockets _weaponactor)
    (Utilities|Map|Add (Variables|Tracing|GetWeaponSocketLastLocation) _array_element (Transformation|GetSocketLocation (Variables|/Game/1Game/Weapons/BP_Base_SWeapon.BP_Base_SWeapon_C|GetWeapon _weaponactor) _array_element))
    (Utilities|Map|Add (Variables|Tracing|GetWeaponSocketLastLastLocation) _array_element (Transformation|GetSocketLocation (Variables|/Game/1Game/Weapons/BP_Base_SWeapon.BP_Base_SWeapon_C|GetWeapon _weaponactor) _array_element))))

(fn GetDirectionOfAnotherActor
  (params (TargetActor :type Actor%20Object%20Reference) (AnotherActor :type Actor%20Object%20Reference))
  (bind _returnvalue (Transformation|GetActorForwardVector AnotherActor))
  (bind _returnvalue_2 (Transformation|GetActorForwardVector TargetActor))
  (bind _returnvalue_3 (Transformation|GetActorLocation AnotherActor))
  (bind _returnvalue_4 (Transformation|GetActorLocation TargetActor))
  (bind _returnvalue_5 (Transformation|GetActorRightVector TargetActor))
  (bind _returnvalue_6 (Math|Vector|Normalize _returnvalue))
  (bind _returnvalue_7 (Math|Vector|Normalize _returnvalue_2))
  (bind _returnvalue_8 (- _returnvalue_4 _returnvalue_3))
  (bind _returnvalue_9 (Math|Vector|DotProduct _returnvalue_7 _returnvalue_6))
  (bind _returnvalue_10 (Math|Vector|DotProduct _returnvalue_8 _returnvalue_5))
  (if (>= _returnvalue_9 0.6)
    (LocalVariables|SetReturnValueDirection "NewEnumerator0")
    (elif (<= _returnvalue_9 -0.8)
      (LocalVariables|SetReturnValueDirection "NewEnumerator3")
      (elif (> _returnvalue_10 0.0)
        (LocalVariables|SetReturnValueDirection "NewEnumerator2")
        (elif (< _returnvalue_10 0.0)
          (LocalVariables|SetReturnValueDirection "NewEnumerator1")
          (else
            (LocalVariables|SetReturnValueDirection "NewEnumerator0"))))))
  (return (LocalVariables|GetReturnValueDirection)))

(fn AfterEquip
  (bind _character (Variables|Default|GetCharacter))
  (Default|SetMovementRotationType _character true)
  (Default|SetBSto _character (Variables|/Game/1Game/Weapons/BP_Base_SWeapon.BP_Base_SWeapon_C|GetBSType (Variables|Default|GetWeaponActor)))
  (Variables|States|SetIsWeaponEquipped? true))

(fn AfterDequip
  (bind _character (Variables|Default|GetCharacter))
  (Variables|States|SetIsWeaponEquipped? false)
  (Default|SetMovementRotationType _character false)
  (Variables|States|SetDequipAlreadyStarted? false)
  (Default|SetBSto _character "NewEnumerator0"))