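; AC_BlockSystem is an actor component that handles the blocking state of its owning BP_YukoPawn.
; On BeginPlay it casts and caches the owner as Character.
; BlockStart sets IsBlocking, saves the current speed mode and switches the pawn to a blocking speed mode.
; BlockEnd restores the saved mode and clears IsBlocking only if the pawn is still in that blocking mode.
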(event Custom|BlockStart
  (bind _character (Variables|Default|GetCharacter))
  (Variables|Default|SetIsBlocking? true)
  (Variables|Default|SetSpeedModeBeforeBlock (Variables|/Game/YukoProject/Character/Blueprints/BP_YukoPawn.BP_YukoPawn_C|GetCurrentSpeedMode _character))
  (Default|SetCharacterSpeedMode _character "NewEnumerator5"))

(event Custom|BlockEnd
  (bind _character (Variables|Default|GetCharacter))
  (if (Utilities|Enum|Equal(Enum) (Variables|/Game/YukoProject/Character/Blueprints/BP_YukoPawn.BP_YukoPawn_C|GetCurrentSpeedMode _character) "NewEnumerator5")
    (Default|SetCharacterSpeedMode _character (Variables|Default|GetSpeedModeBeforeBlock))
    (Variables|Default|SetIsBlocking? false)))

(event EventBeginPlay
  (bind _asbp_yuko_pawn (Utilities|Casting|CastToBP_YukoPawn (Components|GetOwner)))
  (Variables|Default|SetCharacter _asbp_yuko_pawn))