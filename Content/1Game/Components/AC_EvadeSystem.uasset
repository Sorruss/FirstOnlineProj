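; Evade component for BP_YukoPawn that plays an eight-way dodge when a weapon is equipped and a forward roll otherwise.
; A DoOnce gate blocks repeat evades, setting the evading flag and animation lock until a montage notify clears them and reopens it.
; Dodge montages are selected from exact movement X/Y values read through BPI_EvadeSystem, with Forward as the fallback when the interface is absent.
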(event Custom|Evade8Way
  (bind _character (Variables|Default|GetCharacter))
  ;[0.15 0.15 0.15 0.5] Dodge Eight-Way Evade
  (bind _notifyname (Animation|Montage|PlayMontage (Variables|/Script/Engine.Character|GetMesh _character) (Utilities|Select :Index (CallFunction|GetPlayerMovementDirection _character) :NewEnumerator8 0 :NewEnumerator0 "/Game/1Game/Animations/MC/Weapons/Sword/KatanaAnimset/Evade/DodgeForward_Root_Montage.DodgeForward_Root_Montage" :NewEnumerator1 "/Game/1Game/Animations/MC/Weapons/Sword/KatanaAnimset/Evade/DodgeForwardRight_Root_Montage.DodgeForwardRight_Root_Montage" :NewEnumerator2 "/Game/1Game/Animations/MC/Weapons/Sword/KatanaAnimset/Evade/DodgeForwardLeft_Root_Montage.DodgeForwardLeft_Root_Montage" :NewEnumerator3 "/Game/1Game/Animations/MC/Weapons/Sword/KatanaAnimset/Evade/DodgeBack_Root_Montage.DodgeBack_Root_Montage" :NewEnumerator4 "/Game/1Game/Animations/MC/Weapons/Sword/KatanaAnimset/Evade/DodgeBackRight_Root_Montage.DodgeBackRight_Root_Montage" :NewEnumerator5 "/Game/1Game/Animations/MC/Weapons/Sword/KatanaAnimset/Evade/DodgeBackLeft_Root_Montage.DodgeBackLeft_Root_Montage" :NewEnumerator6 "/Game/1Game/Animations/MC/Weapons/Sword/KatanaAnimset/Evade/DodgeRight_Root_Montage.DodgeRight_Root_Montage" :NewEnumerator7 "/Game/1Game/Animations/MC/Weapons/Sword/KatanaAnimset/Evade/DodgeLeft_Root_Montage.DodgeLeft_Root_Montage"))
    (:OnNotifyBegin
      (switch name _notifyname
        (:AnimationLockOff
          (CallFunction|EvadeGateReset))))))

(event Custom|EvadeForwardRoll
  ;[0.15 0.15 0.15 0.5] Roll One-Way Evade
  (bind _notifyname (Animation|Montage|PlayMontage (Variables|/Script/Engine.Character|GetMesh (Variables|Default|GetCharacter)) "/Game/1Game/Animations/MC/Locomotion/AL_Standard_Anim_Rig_Roll_RM_Montage.AL_Standard_Anim_Rig_Roll_RM_Montage")
    (:OnNotifyBegin
      (switch name _notifyname
        (:AnimationLockOff
          (CallFunction|EvadeGateReset))))))

(event Custom|Evade
  ;[0.15 0.15 0.15 0.5] Evade Activation Logic
  (Utilities|FlowControl|DoOnce false
    (:Completed
      (Variables|Default|SetIsEvading? true)
      (Default|SetAnimationLock (Variables|Default|GetCharacter) true)
      (if (Variables|/Game/1Game/Components/AC_AttackSystem.AC_AttackSystem_C|GetIsWeaponEquipped? (Variables|/Game/YukoProject/Character/Blueprints/BP_YukoPawn.BP_YukoPawn_C|GetAC_AttackSystem (Variables|Default|GetCharacter)))
        (CallFunction|Evade8Way)
        (else
          (CallFunction|EvadeForwardRoll))))))

(event Custom|EvadeGateReset
  ;[0.15 0.15 0.15 0.5] Evade Activation Logic
  (Default|SetAnimationLock (Variables|Default|GetCharacter) false)
  (Variables|Default|SetIsEvading? false)
  (Utilities|FlowControl|DoOnce false) ; enters at Reset
)

(event EventBeginPlay
  (bind _asbp_yuko_pawn (Utilities|Casting|CastToBP_YukoPawn (Components|GetOwner)))
  (Variables|Default|SetCharacter _asbp_yuko_pawn))

(fn GetPlayerMovementDirection
  (params (Actor :type Actor%20Object%20Reference))
  (if (Utilities|DoesObjectImplementInterface Actor "/Game/1Game/Controls/Interfaces/BPI_EvadeSystem.BPI_EvadeSystem_C")
    (bind (_movementx _movementy) (Class|BPIEvadeSystem|GetMovementXY(Message) Actor))
    (LocalVariables|SetX _movementx)
    (LocalVariables|SetY _movementy)
    (if (== (LocalVariables|GetX) 1.0)
      (if (== (LocalVariables|GetY) 0.0)
        (return "NewEnumerator6")
        (elif (== (LocalVariables|GetY) 1.0)
          (return "NewEnumerator1")
          (else
            (return "NewEnumerator4"))))
      (elif (== (LocalVariables|GetX) 0.0)
        (if (== (LocalVariables|GetY) 0.0)
          (return "NewEnumerator8")
          (elif (== (LocalVariables|GetY) 1.0)
            (return "NewEnumerator0")
            (else
              (return "NewEnumerator3"))))
        (elif (== (LocalVariables|GetX) -1.0)
          (if (== (LocalVariables|GetY) 0.0)
            (return "NewEnumerator7")
            (elif (== (LocalVariables|GetY) 1.0)
              (return "NewEnumerator2")
              (else
                (return "NewEnumerator5")))))))
    (else
      (return "NewEnumerator0"))))