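; Game mode Blueprint, by its name for the replication part of the game, that spawns or respawns players as BP_YukoPawn.
; SpawnPlayer destroys the controller's current pawn, spawns a new one regardless of collision, and possesses it with that controller.
; FindRandomPlayerStartTransform supplies the spawn location and rotation by picking randomly among all PlayerStart actors in the level.
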(event Custom|SpawnPlayer
  (params (PlayerController :type Player%20Controller%20Object%20Reference))
  (bind _returnvalue (Pawn|GetControlledPawn PlayerController))
  (bind _transform (CallFunction|FindRandomPlayerStartTransform))
  (Utilities|IsValid _returnvalue
    (:Is%20Valid
      (Actor|DestroyActor _returnvalue))
    (:Is%20Not%20Valid
      _))
  (bind _returnvalue_2 (Game|SpawnActorfromClass "/Game/YukoProject/Character/Blueprints/BP_YukoPawn.BP_YukoPawn_C" (Math|Transform|MakeTransform (.location _transform) (.rotation _transform) "1.000000,1.000000,1.000000") "AlwaysSpawn" "MultiplyWithRoot" 0 0))
  (Pawn|Possess PlayerController _returnvalue_2))

(fn ConstructionScript)

(fn FindRandomPlayerStartTransform
  (bind _outactors (Actor|GetAllActorsOfClass "/Script/Engine.PlayerStart"))
  (return (Transformation|GetActorTransform (Utilities|Array|Get(acopy) _outactors (Math|Random|RandomIntegerinRange 0 (- (Utilities|Array|Length _outactors) 1))))))