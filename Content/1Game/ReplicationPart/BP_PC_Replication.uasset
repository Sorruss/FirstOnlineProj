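; BP_PC_Replication is a player controller that requests its player's spawn from the game mode in a networked game.
; On BeginPlay, only the local controller fires SpawnPlayer, which forwards the request through ROS_SpawnPlayer, apparently a run-on-server event.
; With authority, that event casts the game mode to BP_GM_Replication and calls its SpawnPlayer with this controller, leaving the spawn logic to the game mode.
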(event Custom|ROS_SpawnPlayer
  (Networking|SwitchHasAuthority
    (:Authority
      (bind _asbp_gm_replication (Utilities|Casting|CastToBP_GM_Replication (Game|GetGameMode)))
      (Default|SpawnPlayer _asbp_gm_replication self))))

(event Custom|SpawnPlayer
  (CallFunction|ROSSpawnPlayer))

(event EventBeginPlay
  (if (Pawn|IsLocalPlayerController)
    (CallFunction|SpawnPlayer)))

(fn ConstructionScript)